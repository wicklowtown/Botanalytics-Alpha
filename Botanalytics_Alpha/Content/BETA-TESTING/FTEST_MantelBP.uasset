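; Functional test Blueprint that, going by its name, checks character mantling by driving a referenced character toward a trigger.
; Tick constantly feeds forward movement input to the character, and StartTest makes it jump after a short delay.
; The test succeeds when that character begins overlapping the trigger actor; the graph itself defines no failure path.
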(event OnActorBeginOverlap(Tr1gger)
  (params (OverlappedActor :type Actor%20Object%20Reference) (OtherActor :type Actor%20Object%20Reference))
  (if (== OtherActor (Variables|Default|GetCharacterr))
    (Class|FunctionalTest|FinishTest "Succeeded")))

(event EventPrepareTest)

(event EventStartTest
  (Utilities|FlowControl|Delay 0.5)
  (Character|Jump (Variables|Default|GetCharacterr)))

(event EventTick
  (params (DeltaSeconds :type Float%20%28single-precision%29))
  (bind _characterr (Variables|Default|GetCharacterr))
  (Pawn|Input|AddMovementInput _characterr (Transformation|GetActorForwardVector _characterr) 5.0 false))

(fn ConstructionScript)