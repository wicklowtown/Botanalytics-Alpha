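; BP_Flowers is a morph target demo that grows three flowers in steps on key presses.
; Pressing G plays a separate timeline per flower that still has growth left, scaling its curve by 0.2 and adding it to that flower's stored value to drive the "Growing" morph target.
; Each timeline saves the new value when finished, so growth accumulates across presses.
; Pressing R resets all three morphs and stored values to zero.
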(event Input|KeyboardEvents|R
  (params (Key :type Key%20Structure :default "None"))
  (:Pressed
    (Components|SkeletalMesh|SetMorphTarget (Variables|Default|GetFlower%2002) "Growing" 0.0 true)
    (Variables|Default|SetGrowing%2001 0.0)
    (Variables|Default|SetGrowing%2002 0.0)
    (Variables|Default|SetGrowing%2003 0.0)))

(event Input|KeyboardEvents|G
  (params (Key :type Key%20Structure :default "None"))
  (:Pressed
    (Utilities|FlowControl|Sequence
      (:then_0
        (if (< (Variables|Default|GetGrowing%2001) 1.0)
          (bind _growing (Timeline|Grow%2001 PlayFromStart)
            (:Update
              (Components|SkeletalMesh|SetMorphTarget (Variables|Default|GetFlower%2001) "Growing" (+ (Variables|Default|GetGrowing%2001) (* _growing 0.2)) true))
            (:Finished
              (Variables|Default|SetGrowing%2001 (+ (Variables|Default|GetGrowing%2001) (* _growing 0.2)))))))
      (:then_1
        (if (< (Variables|Default|GetGrowing%2002) 1.0)
          (bind _growing_2 (Timeline|Grow%2002 PlayFromStart)
            (:Update
              (Components|SkeletalMesh|SetMorphTarget (Variables|Default|GetFlower%2002) "Growing" (+ (Variables|Default|GetGrowing%2002) (* _growing_2 0.2)) true))
            (:Finished
              (Variables|Default|SetGrowing%2002 (+ (Variables|Default|GetGrowing%2002) (* _growing_2 0.2)))))))
      (:then_2
        (if (< (Variables|Default|GetGrowing%2003) 1.0)
          (bind _growing_3 (Timeline|Grow%2003 PlayFromStart)
            (:Update
              (Components|SkeletalMesh|SetMorphTarget (Variables|Default|GetFlower%2003) "Growing" (+ (Variables|Default|GetGrowing%2003) (* _growing_3 0.2)) true))
            (:Finished
              (Variables|Default|SetGrowing%2003 (+ (Variables|Default|GetGrowing%2003) (* _growing_3 0.2))))))))))

(fn ConstructionScript)